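; Menu HUD that draws a radial main menu on the canvas and prints the WaveController's current beat.
; The construction script caches the first WaveController in the level, and DrawHUD passes hard-coded labels to DrawRadialMenu through a Gate.
; Nine textured buttons sit at the centre and eight compass offsets, with text centred on non-empty labels.
; Buttons are display-only: no input handling, and hover and pressed textures go unused.
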(event `self.ReceiveDrawHUD`
  (params (SizeX :type Integer) (SizeY :type Integer))
  (`self.DrawText` (`KismetStringLibrary.Conv_IntToString` (`/Game/Blueprints/WaveUtilities/WaveController.CurrentBeat` (`self.WaveController`))) (struct :`G` 0.018932 :`B` 0.325 :`A` 1.0) 0.0 0.0 "/Game/MenuFont.MenuFont")
  (`/Engine/EditorBlueprintResources/StandardMacros.Gate` true
    (:`Exit`
      (bind _options (`self.Create Main Menu Options`))
      (`self.Draw Radial Menu` _options (`KismetMathLibrary.MakeVector2D` (/ (`KismetMathLibrary.Conv_IntToDouble` SizeX) 2.0) (/ (`KismetMathLibrary.Conv_IntToDouble` SizeY) 2.0))))))

(fn `Create Main Menu Options`
  (returns (Options :type "Array of String"))
  (return (`|MakeArray` "Back" "New Game" "" "Select Level" "" "Quit" "Extras" "Options" "")))

(fn `Draw Button`
  (params (Text :type String) (`Up Texture` :type "Texture2D Object Reference") (`Over Texture` :type "Texture2D Object Reference") (`Down Texture` :type "Texture2D Object Reference") (Coordinates :type "Object.Vector2D Structure") (`Screen Center` :type "Object.Vector2D Structure"))
  (bind _font_scale (`self.Font Scale`))
  (bind (_position _size) (`self.Get Button Bounds` Coordinates `Screen Center` `Up Texture`))
  (bind (_x _y) (`KismetMathLibrary.BreakVector2D` _position))
  (bind (_x_2 _y_2) (`KismetMathLibrary.BreakVector2D` _size))
  (`self.DrawTexture` `Up Texture` _x _y _x_2 _y_2 0.0 0.0 1.0 1.0)
  (if (not (== Text ""))
    (bind _position_2 (`self.Get Button Text Position` Coordinates _position _size Text _font_scale))
    (bind (_x_3 _y_3) (`KismetMathLibrary.BreakVector2D` _position_2))
    (`self.DrawText` Text (struct :`R` 0.8 :`G` 0.841422 :`B` 1.0 :`A` 1.0) _x_3 _y_3 "/Game/MenuFont.MenuFont" _font_scale)))

(fn `Draw Radial Menu`
  (params (Options :type "Array of String") (`Screen Center` :type "Object.Vector2D Structure"))
  (for (_array_element _array_index) Options
    (`self.Draw Button` _array_element (`KismetArrayLibrary.Array_Get` (`self.Radial Textures`) _array_index) null null (`KismetArrayLibrary.Array_Get` (`|MakeArray` (0.0 0.0) (0.0 1.0) (-1.0 1.0) (-1.0 0.0) (-1.0 -1.0) (0.0 -1.0) (1.0 -1.0) (1.0 0.0) (1.0 1.0) :!type "Object.Vector2D Structure") _array_index) `Screen Center`)))

(fn `Get Button Bounds`
  (params (Coordinates :type "Object.Vector2D Structure") (`Screen Center` :type "Object.Vector2D Structure") (`Ref Texture` :type "Texture2D Object Reference"))
  (returns (Position :type "Object.Vector2D Structure") (Size :type "Object.Vector2D Structure"))
  (bind _returnvalue (`Texture2D.Blueprint_GetSizeX` `Ref Texture`))
  (bind _returnvalue_2 (`Texture2D.Blueprint_GetSizeY` `Ref Texture`))
  (bind (_x _y) (`KismetMathLibrary.BreakVector2D` `Screen Center`))
  (bind (_x_2 _y_2) (`KismetMathLibrary.BreakVector2D` Coordinates))
  (return (`KismetMathLibrary.MakeVector2D` (+ (`KismetMathLibrary.Conv_IntToDouble` (* (/ _returnvalue 2) (- (`KismetMathLibrary.FFloor` _x_2) 1))) (+ _x (* _x_2 -400.0))) (+ (`KismetMathLibrary.Conv_IntToDouble` (* (/ _returnvalue_2 2) (- (`KismetMathLibrary.FFloor` _y_2) 1))) (+ _y (* _y_2 -400.0)))) (`KismetMathLibrary.MakeVector2D` (`KismetMathLibrary.Conv_IntToDouble` _returnvalue) (`KismetMathLibrary.Conv_IntToDouble` _returnvalue_2))))

(fn `Get Button Text Position`
  (params (Coordinates :type "Object.Vector2D Structure") (`Button Position` :type "Object.Vector2D Structure") (`Button Size` :type "Object.Vector2D Structure") (Text :type String) (`Font Scale` :type "Float (double-precision)"))
  (returns (Position :type "Object.Vector2D Structure"))
  (bind (_x _y) (`KismetMathLibrary.BreakVector2D` `Button Position`))
  (bind (_x_2 _y_2) (`KismetMathLibrary.BreakVector2D` `Button Size`))
  (bind (_outwidth _outheight) (`self.GetTextSize` Text "/Game/MenuFont.MenuFont" `Font Scale`))
  (return (`KismetMathLibrary.MakeVector2D` (- (+ _x (/ _x_2 2.0)) (/ _outwidth 2.0)) (- (+ _y (/ _y_2 2.0)) (/ _outheight 2.0)))))

(fn `UserConstructionScript`
  (bind _outactors (`GameplayStatics.GetAllActorsOfClass` "/Game/Blueprints/WaveUtilities/WaveController.WaveController_C"))
  (bind _aswavecontroller_c (cast `/Game/Blueprints/WaveUtilities/WaveController` (`KismetArrayLibrary.Array_Get` _outactors)))
  (set `self.WaveController` _aswavecontroller_c))