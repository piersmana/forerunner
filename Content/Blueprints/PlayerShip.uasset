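; Player ship for a beat-driven grid dodging game, synced to WaveController's beats and level events.
; Held directions pick a grid cell, and timelines lerp the ship there with tilt and bobbing.
; Beat collision checks deal damage or turn grazes into boost, which raises tempo while spent.
; Dynamic materials display damage and boost; death or victory stops the track on a beat and flies the ship away.
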(event Custom|PlayerDies
  (bind _goalrotation (Variables|Default|GetGoalRotation))
  (bind _shipbody (Variables|Default|GetShipBody))
  (Utilities|FlowControl|Sequence
    (:then_0
      (Utilities|FlowControl|Sequence
        (:then_0
          (bind _position (Timeline|GridMovement Stop)
            (:Update
              (Transformation|SetRelativeLocation _shipbody (+ (stale _bobbing) (Math|Vector|Lerp(Vector) (Variables|Default|GetStartLocation) (Variables|Default|GetGoalLocation) _position)) false :!label _label))))
        (:then_1
          (bind _rotation (Timeline|GridRotation Stop)
            (:Update
              (Transformation|SetRelativeRotation _shipbody (Math|Rotator|Lerp(Rotator) (Variables|Default|GetStartRotation) _goalrotation _rotation true) false))
            (:Finished
              (bind _rotation_2 (Timeline|GridRot2 PlayFromStart)
                (:Update
                  (Transformation|SetRelativeRotation _shipbody (Math|Rotator|Lerp(Rotator) "0, 0, 0" _goalrotation _rotation_2 true) false))))))
        (:then_2
          (Timeline|GridRot2 Stop))
        (:then_3
          ;[1 1 1] Controls Passive Bobbing Motion
          (bind _bobbing (Timeline|Bobbing%20motion Stop)
            (:Update
              (goto _label))))
        (:then_4
          (Input|DisableInput 0)
          (Variables|Default|SetStartLocation (Variables|/Script/Engine.SceneComponent|GetRelativeLocation _shipbody))
          (Variables|Default|SetStartRotation (Variables|/Script/Engine.SceneComponent|GetRelativeRotation _shipbody)))))
    (:then_1
      (EventDispatchers|BindEventtoAdvanceBeat (Variables|Default|GetWaveController) (delegate Custom|FinBeat)))))

(event Custom|PlayerWins
  (bind _goalrotation (Variables|Default|GetGoalRotation))
  (bind _shipbody (Variables|Default|GetShipBody))
  (Utilities|FlowControl|Sequence
    (:then_0
      (Utilities|FlowControl|Sequence
        (:then_0
          (bind _position (Timeline|GridMovement Stop)
            (:Update
              (Transformation|SetRelativeLocation _shipbody (+ (stale _bobbing) (Math|Vector|Lerp(Vector) (Variables|Default|GetStartLocation) (Variables|Default|GetGoalLocation) _position)) false :!label _label))))
        (:then_1
          (bind _rotation (Timeline|GridRotation Stop)
            (:Update
              (Transformation|SetRelativeRotation _shipbody (Math|Rotator|Lerp(Rotator) (Variables|Default|GetStartRotation) _goalrotation _rotation true) false))
            (:Finished
              (bind _rotation_2 (Timeline|GridRot2 PlayFromStart)
                (:Update
                  (Transformation|SetRelativeRotation _shipbody (Math|Rotator|Lerp(Rotator) "0, 0, 0" _goalrotation _rotation_2 true) false))))))
        (:then_2
          (Timeline|GridRot2 Stop))
        (:then_3
          ;[1 1 1] Controls Passive Bobbing Motion
          (bind _bobbing (Timeline|Bobbing%20motion Stop)
            (:Update
              (goto _label))))
        (:then_4
          (Input|DisableInput 0)
          (Variables|Default|SetStartLocation (Variables|/Script/Engine.SceneComponent|GetRelativeLocation _shipbody))
          (Variables|Default|SetStartRotation (Variables|/Script/Engine.SceneComponent|GetRelativeRotation _shipbody)))))
    (:then_1
      (EventDispatchers|BindEventtoAdvanceBeat (Variables|Default|GetWaveController) (delegate Custom|WinBeat)))))

(event Custom|BeginGameplay_Event
  (Input|EnableInput (Game|GetPlayerController 0)))

(event Custom|NewBeat
  (params (NewBeat :type Integer) (IsDownBeat :type Boolean))
  (CallFunction|HandleCollision true))

(event Custom|WinBeat
  (params (NewBeat :type Integer) (IsDownBeat :type Boolean))
  (bind _shipbody (Variables|Default|GetShipBody))
  (Default|StopTrack (Variables|Default|GetWaveController) false)
  (bind _position (Timeline|Timeline_1 Play)
    (:Update
      (Transformation|SetRelativeLocation _shipbody (Math|Vector|Lerp(Vector) (Variables|Default|GetStartLocation) "0.000000,3600.000000,200.000000" _position) false)
      (Transformation|SetRelativeRotation _shipbody (Math|Rotator|Lerp(Rotator) (Variables|Default|GetStartRotation) "0.000000,0.000000,-60.000000" _position true) false))
    (:Finished
      (Rendering|SetActorHiddenInGame true))))

(event Custom|FinBeat
  (params (NewBeat :type Integer) (IsDownBeat :type Boolean))
  (bind _shipbody (Variables|Default|GetShipBody))
  (Default|StopTrack (Variables|Default|GetWaveController) true)
  (bind _position (Timeline|Timeline_0 Play)
    (:Update
      (Transformation|SetRelativeLocation _shipbody (Math|Vector|Lerp(Vector) (Variables|Default|GetStartLocation) "10.000000,1200.000000,-50.000000" _position) false)
      (Transformation|SetRelativeRotation _shipbody (Math|Rotator|Lerp(Rotator) (Variables|Default|GetStartRotation) "170.000000,90.000000, 0" _position true) false))
    (:Finished
      (Rendering|SetActorHiddenInGame true))))

(event EventBeginPlay
  (bind _wavecontroller (Variables|Default|GetWaveController))
  (Input|DisableInput 0)
  (EventDispatchers|BindEventtoLevelComplete _wavecontroller (delegate Custom|PlayerWins))
  (EventDispatchers|BindEventtoBeginGameplay _wavecontroller (delegate Custom|BeginGameplay_Event))
  (EventDispatchers|BindEventtoAdvanceBeatB _wavecontroller (delegate Custom|NewBeat))
  (bind (_loc_x _loc_z) (Default|GetLocationfromGrid _wavecontroller "NewEnumerator4"))
  (Variables|Default|SetGoalLocation (Math|Vector|MakeVector _loc_x 0.0 _loc_z)))

(event EventTick
  (params (DeltaSeconds :type Float%20%28single-precision%29))
  (bind _wavecontroller (Variables|Default|GetWaveController))
  (if (Variables|Controls|GetTryBoost)
    (CallFunction|ConsumeBoost)
    (if (Variables|State|GetBoosting)
      (Utilities|FlowControl|Sequence
        (:then_0
          (Utilities|FlowControl|DoOnce false :!label _label
            (:Completed
              (Default|IncreaseTempo _wavecontroller))))
        (:then_1
          (goto _label_3 Reset)))
      (else
        (Utilities|FlowControl|Sequence :!label _label_2
          (:then_0
            (Utilities|FlowControl|DoOnce true :!label _label_3
              (:Completed
                (Default|ResetTempo _wavecontroller))))
          (:then_1
            (goto _label Reset)))))
    (else
      (goto _label_2))))

(event Input|ActionEvents|InputActionBoost
  (:Pressed
    (Variables|Controls|SetTryBoost true)
    (CallFunction|ConsumeBoost)
    (if (Variables|State|GetBoosting)
      _))
  (:Released
    (Variables|Controls|SetTryBoost false)))

(event Input|ActionEvents|InputActionRight
  (bind _wavecontroller (Variables|Default|GetWaveController))
  (bind _shipbody (Variables|Default|GetShipBody))
  (:Pressed
    (Variables|Controls|SetRight true)
    (if (not false) :!label _label
      (Variables|Movement|SetPrevGridPosition (Variables|Movement|GetGridPosition))
      (Variables|Movement|SetGridPosition (CallFunction|GetNewGridPosition))
      (bind (_loc_x _loc_z) (Default|GetLocationfromGrid _wavecontroller (Variables|Movement|GetGridPosition)))
      (Variables|Default|SetGoalLocation (Math|Vector|MakeVector _loc_x 0.0 _loc_z))
      (bind (_loc_x_2 _loc_z_2) (Default|GridNametoValues _wavecontroller (Variables|Movement|GetGridPosition)))
      (bind (_loc_x_3 _loc_z_3) (Default|GridNametoValues _wavecontroller (Variables|Movement|GetPrevGridPosition)))
      (Variables|Default|SetGoalRotation (Class|KismetMathLibrary|MakeRot (* (- _loc_x_3 _loc_x_2) (Variables|Movement|GetPitchValue)) (* (- _loc_x_3 _loc_x_2) (Variables|Movement|GetPitchValue)) (* (- _loc_z_3 _loc_z_2) (Variables|Movement|GetRollValue))))
      (Variables|Default|SetStartLocation (Variables|/Script/Engine.SceneComponent|GetRelativeLocation _shipbody))
      (Variables|Default|SetStartRotation (Variables|/Script/Engine.SceneComponent|GetRelativeRotation _shipbody))
      (CallFunction|HandleCollision false)
      (Utilities|FlowControl|Sequence
        (:then_0
          (bind _position (Timeline|GridMovement PlayFromStart)
            (:Update
              (Transformation|SetRelativeLocation _shipbody (+ (stale Custom|PlayerDies _bobbing) (Math|Vector|Lerp(Vector) (Variables|Default|GetStartLocation) (Variables|Default|GetGoalLocation) _position)) false))))
        (:then_1
          (bind _rotation (Timeline|GridRotation PlayFromStart)
            (:Update
              (Transformation|SetRelativeRotation _shipbody (Math|Rotator|Lerp(Rotator) (Variables|Default|GetStartRotation) (Variables|Default|GetGoalRotation) _rotation true) false))
            (:Finished
              (bind _rotation_2 (Timeline|GridRot2 PlayFromStart)
                (:Update
                  (Transformation|SetRelativeRotation _shipbody (Math|Rotator|Lerp(Rotator) "0, 0, 0" (Variables|Default|GetGoalRotation) _rotation_2 true) false))))))
        (:then_2
          (Timeline|GridRot2 Stop)))))
  (:Released
    (Variables|Controls|SetRight false)
    (goto _label)))

(event Input|ActionEvents|InputActionLeft
  (bind _wavecontroller (Variables|Default|GetWaveController))
  (bind _shipbody (Variables|Default|GetShipBody))
  (:Pressed
    (Variables|Controls|SetLeft true)
    (if (not false) :!label _label
      (Variables|Movement|SetPrevGridPosition (Variables|Movement|GetGridPosition))
      (Variables|Movement|SetGridPosition (CallFunction|GetNewGridPosition))
      (bind (_loc_x _loc_z) (Default|GetLocationfromGrid _wavecontroller (Variables|Movement|GetGridPosition)))
      (Variables|Default|SetGoalLocation (Math|Vector|MakeVector _loc_x 0.0 _loc_z))
      (bind (_loc_x_2 _loc_z_2) (Default|GridNametoValues _wavecontroller (Variables|Movement|GetGridPosition)))
      (bind (_loc_x_3 _loc_z_3) (Default|GridNametoValues _wavecontroller (Variables|Movement|GetPrevGridPosition)))
      (Variables|Default|SetGoalRotation (Class|KismetMathLibrary|MakeRot (* (- _loc_x_3 _loc_x_2) (Variables|Movement|GetPitchValue)) (* (- _loc_x_3 _loc_x_2) (Variables|Movement|GetPitchValue)) (* (- _loc_z_3 _loc_z_2) (Variables|Movement|GetRollValue))))
      (Variables|Default|SetStartLocation (Variables|/Script/Engine.SceneComponent|GetRelativeLocation _shipbody))
      (Variables|Default|SetStartRotation (Variables|/Script/Engine.SceneComponent|GetRelativeRotation _shipbody))
      (CallFunction|HandleCollision false)
      (Utilities|FlowControl|Sequence
        (:then_0
          (bind _position (Timeline|GridMovement PlayFromStart)
            (:Update
              (Transformation|SetRelativeLocation _shipbody (+ (stale Custom|PlayerDies _bobbing) (Math|Vector|Lerp(Vector) (Variables|Default|GetStartLocation) (Variables|Default|GetGoalLocation) _position)) false))))
        (:then_1
          (bind _rotation (Timeline|GridRotation PlayFromStart)
            (:Update
              (Transformation|SetRelativeRotation _shipbody (Math|Rotator|Lerp(Rotator) (Variables|Default|GetStartRotation) (Variables|Default|GetGoalRotation) _rotation true) false))
            (:Finished
              (bind _rotation_2 (Timeline|GridRot2 PlayFromStart)
                (:Update
                  (Transformation|SetRelativeRotation _shipbody (Math|Rotator|Lerp(Rotator) "0, 0, 0" (Variables|Default|GetGoalRotation) _rotation_2 true) false))))))
        (:then_2
          (Timeline|GridRot2 Stop)))))
  (:Released
    (Variables|Controls|SetLeft false)
    (goto _label)))

(event Input|ActionEvents|InputActionDown
  (bind _wavecontroller (Variables|Default|GetWaveController))
  (bind _shipbody (Variables|Default|GetShipBody))
  (:Pressed
    (Variables|Controls|SetDown true)
    (if (not false) :!label _label
      (Variables|Movement|SetPrevGridPosition (Variables|Movement|GetGridPosition))
      (Variables|Movement|SetGridPosition (CallFunction|GetNewGridPosition))
      (bind (_loc_x _loc_z) (Default|GetLocationfromGrid _wavecontroller (Variables|Movement|GetGridPosition)))
      (Variables|Default|SetGoalLocation (Math|Vector|MakeVector _loc_x 0.0 _loc_z))
      (bind (_loc_x_2 _loc_z_2) (Default|GridNametoValues _wavecontroller (Variables|Movement|GetGridPosition)))
      (bind (_loc_x_3 _loc_z_3) (Default|GridNametoValues _wavecontroller (Variables|Movement|GetPrevGridPosition)))
      (Variables|Default|SetGoalRotation (Class|KismetMathLibrary|MakeRot (* (- _loc_x_3 _loc_x_2) (Variables|Movement|GetPitchValue)) (* (- _loc_x_3 _loc_x_2) (Variables|Movement|GetPitchValue)) (* (- _loc_z_3 _loc_z_2) (Variables|Movement|GetRollValue))))
      (Variables|Default|SetStartLocation (Variables|/Script/Engine.SceneComponent|GetRelativeLocation _shipbody))
      (Variables|Default|SetStartRotation (Variables|/Script/Engine.SceneComponent|GetRelativeRotation _shipbody))
      (CallFunction|HandleCollision false)
      (Utilities|FlowControl|Sequence
        (:then_0
          (bind _position (Timeline|GridMovement PlayFromStart)
            (:Update
              (Transformation|SetRelativeLocation _shipbody (+ (stale Custom|PlayerDies _bobbing) (Math|Vector|Lerp(Vector) (Variables|Default|GetStartLocation) (Variables|Default|GetGoalLocation) _position)) false))))
        (:then_1
          (bind _rotation (Timeline|GridRotation PlayFromStart)
            (:Update
              (Transformation|SetRelativeRotation _shipbody (Math|Rotator|Lerp(Rotator) (Variables|Default|GetStartRotation) (Variables|Default|GetGoalRotation) _rotation true) false))
            (:Finished
              (bind _rotation_2 (Timeline|GridRot2 PlayFromStart)
                (:Update
                  (Transformation|SetRelativeRotation _shipbody (Math|Rotator|Lerp(Rotator) "0, 0, 0" (Variables|Default|GetGoalRotation) _rotation_2 true) false))))))
        (:then_2
          (Timeline|GridRot2 Stop)))))
  (:Released
    (Variables|Controls|SetDown false)
    (goto _label)))

(event Input|ActionEvents|InputActionUp
  (bind _wavecontroller (Variables|Default|GetWaveController))
  (bind _shipbody (Variables|Default|GetShipBody))
  (:Pressed
    (Variables|Controls|SetUp true)
    (if (not false) :!label _label
      (Variables|Movement|SetPrevGridPosition (Variables|Movement|GetGridPosition))
      (Variables|Movement|SetGridPosition (CallFunction|GetNewGridPosition))
      (bind (_loc_x _loc_z) (Default|GetLocationfromGrid _wavecontroller (Variables|Movement|GetGridPosition)))
      (Variables|Default|SetGoalLocation (Math|Vector|MakeVector _loc_x 0.0 _loc_z))
      (bind (_loc_x_2 _loc_z_2) (Default|GridNametoValues _wavecontroller (Variables|Movement|GetGridPosition)))
      (bind (_loc_x_3 _loc_z_3) (Default|GridNametoValues _wavecontroller (Variables|Movement|GetPrevGridPosition)))
      (Variables|Default|SetGoalRotation (Class|KismetMathLibrary|MakeRot (* (- _loc_x_3 _loc_x_2) (Variables|Movement|GetPitchValue)) (* (- _loc_x_3 _loc_x_2) (Variables|Movement|GetPitchValue)) (* (- _loc_z_3 _loc_z_2) (Variables|Movement|GetRollValue))))
      (Variables|Default|SetStartLocation (Variables|/Script/Engine.SceneComponent|GetRelativeLocation _shipbody))
      (Variables|Default|SetStartRotation (Variables|/Script/Engine.SceneComponent|GetRelativeRotation _shipbody))
      (CallFunction|HandleCollision false)
      (Utilities|FlowControl|Sequence
        (:then_0
          (bind _position (Timeline|GridMovement PlayFromStart)
            (:Update
              (Transformation|SetRelativeLocation _shipbody (+ (stale Custom|PlayerDies _bobbing) (Math|Vector|Lerp(Vector) (Variables|Default|GetStartLocation) (Variables|Default|GetGoalLocation) _position)) false))))
        (:then_1
          (bind _rotation (Timeline|GridRotation PlayFromStart)
            (:Update
              (Transformation|SetRelativeRotation _shipbody (Math|Rotator|Lerp(Rotator) (Variables|Default|GetStartRotation) (Variables|Default|GetGoalRotation) _rotation true) false))
            (:Finished
              (bind _rotation_2 (Timeline|GridRot2 PlayFromStart)
                (:Update
                  (Transformation|SetRelativeRotation _shipbody (Math|Rotator|Lerp(Rotator) "0, 0, 0" (Variables|Default|GetGoalRotation) _rotation_2 true) false))))))
        (:then_2
          (Timeline|GridRot2 Stop)))))
  (:Released
    (Variables|Controls|SetUp false)
    (goto _label)))

(fn ConstructionScript
  (bind _shipbody (Variables|Default|GetShipBody))
  (bind _damagestates (Variables|State|GetDamageStates))
  (bind _returnvalue (Rendering|Material|CreateDynamicMaterialInstance _shipbody 2 "/Game/Materials/JetsGlow_Inst.JetsGlow_Inst" :!class /Script/Engine.PrimitiveComponent))
  (bind _returnvalue_2 (Rendering|Material|CreateDynamicMaterialInstance _shipbody 1 "/Game/Materials/JetsGlow_Inst2.JetsGlow_Inst2" :!class /Script/Engine.PrimitiveComponent))
  (bind _returnvalue_3 (Rendering|Material|CreateDynamicMaterialInstance _shipbody 0 "/Game/Materials/JetsGlow_Inst3.JetsGlow_Inst3" :!class /Script/Engine.PrimitiveComponent))
  (bind _returnvalue_4 (Rendering|Material|CreateDynamicMaterialInstance _shipbody 3 "/Game/Materials/JetsGlow_Inst4.JetsGlow_Inst4" :!class /Script/Engine.PrimitiveComponent))
  (Utilities|Array|Add _damagestates _returnvalue)
  (Utilities|Array|Add _damagestates _returnvalue_2)
  (Utilities|Array|Add _damagestates _returnvalue_3)
  (Utilities|Array|Add _damagestates _returnvalue_4)
  (bind _returnvalue_5 (Rendering|Material|CreateDynamicMaterialInstance _shipbody 6 "/Game/Materials/WingsGlow_Inst.WingsGlow_Inst" :!class /Script/Engine.PrimitiveComponent))
  (Variables|State|SetBoostIndicator _returnvalue_5)
  (Rendering|Material|SetScalarParameterValue (Variables|State|GetBoostIndicator) "Intensity" (Variables|State|GetBoostAmount) :!class /Script/Engine.MaterialInstanceDynamic)
  (Rendering|SetVisibility (Variables|Default|GetSpotLight) (Variables|State|GetShowLight) false))

(fn GetNewGridPosition
  (bind _left (Variables|Controls|GetLeft))
  (bind _down (Variables|Controls|GetDown))
  (Utilities|FlowControl|Sequence
    (:then_0
      (if (Variables|Controls|GetRight)
        (if _left
          (LocalVariables|SetHoriz 0 :!label _label)
          (else
            (LocalVariables|SetHoriz -1)))
        (elif _left
          (LocalVariables|SetHoriz 1)
          (else
            (goto _label)))))
    (:then_1
      (if (Variables|Controls|GetUp)
        (if _down
          (LocalVariables|SetVert 0 :!label _label_2)
          (else
            (LocalVariables|SetVert 1)))
        (elif _down
          (LocalVariables|SetVert -1)
          (else
            (goto _label_2)))))
    (:then_2
      (bind _gridposition (Default|GridValuestoName (Variables|Default|GetWaveController) (LocalVariables|GetHoriz) (LocalVariables|GetVert)))
      (return _gridposition))))

(fn HandleCollision
  (params (IsNewBeat :type Boolean))
  (if (not (> (Variables|State|GetDamage) 4))
    (bind _collisiontype (Default|GetGridCollision (Variables|Default|GetWaveController) (Variables|Movement|GetGridPosition)))
    (switch Utilities|FlowControl|Switch|SwitchonEGridState _collisiontype
      (:NewEnumerator0
        (if (and IsNewBeat (Variables|State|GetGrazed))
          (CallFunction|AddBoost)))
      (:NewEnumerator1
        (if (not (Variables|State|GetGrazed))
          (Audio|PlaySoundatLocation "/Game/Sound/graze_a.graze_a" "0, 0, 0")
          (Variables|State|SetGrazed true)))
      (:NewEnumerator2
        (if IsNewBeat
          (CallFunction|TakeDamage))))))

(fn TakeDamage
  (Audio|PlaySoundatLocation "/Game/Sound/chomp.chomp" "0, 0, 0")
  (if (> (Variables|State|GetDamage) 3)
    (CallFunction|PlayerDies))
  (Rendering|Material|SetScalarParameterValue (Utilities|Array|Get(acopy) (Variables|State|GetDamageStates) (Variables|State|GetDamage)) "DamageIndicator" 1.0 :!class /Script/Engine.MaterialInstanceDynamic)
  (Variables|State|SetDamage (+ (Variables|State|GetDamage) 1))
  (CallFunction|LoseBoost))

(fn AddBoost
  (Variables|State|SetBoostAmount (Math|Float|Min(Float) (+ (Variables|State|GetBoostAmount) (Variables|State|GetBoostAddedPerGraze)) (Variables|State|GetMaxBoost)))
  (Audio|PlaySoundatLocation "/Game/Sound/graze_b.graze_b" "0, 0, 0")
  (Variables|State|SetGrazed false)
  (Rendering|Material|SetScalarParameterValue (Variables|State|GetBoostIndicator) "Intensity" (Variables|State|GetBoostAmount) :!class /Script/Engine.MaterialInstanceDynamic))

(fn LoseBoost
  (Variables|State|SetBoostAmount (Math|Float|Max(Float) (- (Variables|State|GetBoostAmount) (Variables|State|GetBoostLostPerHit)) 0.0))
  (Variables|State|SetGrazed false)
  (Rendering|Material|SetScalarParameterValue (Variables|State|GetBoostIndicator) "Intensity" (Variables|State|GetBoostAmount) :!class /Script/Engine.MaterialInstanceDynamic))

(fn ConsumeBoost
  (if (> (Variables|State|GetBoostAmount) 0.0)
    (Variables|State|SetBoostAmount (Math|Float|Max(Float) (- (Variables|State|GetBoostAmount) (* (Variables|State|GetBoostConsumedPerSecond) (Utilities|Time|GetWorldDeltaSeconds))) 0.0))
    (Rendering|Material|SetScalarParameterValue (Variables|State|GetBoostIndicator) "Intensity" (Variables|State|GetBoostAmount) :!class /Script/Engine.MaterialInstanceDynamic)
    (Variables|State|SetBoosting true)
    (else
      (Variables|State|SetBoosting false))))