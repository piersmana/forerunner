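; Construction script for forest_vert, a hazard Blueprint that picks its vertical piece variant from its grid root position.
; After running the parent construction script, it switches on GridRootPosition, with two groups of three positions selecting VertR or VertL.
; The selected component is shown and nudged outward along local X, and the default Vert is hidden.
; Other positions get no changes here.
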(fn `UserConstructionScript`
  (bind _vert (`self.Vert`))
  (bind _vertr (`self.VertR`))
  (bind _vertl (`self.VertL`))
  (`parent.UserConstructionScript`)
  (switch `/Game/Blueprints/WaveUtilities/EGridPosition` (`self.GridRootPosition`)
    (:`NewEnumerator0`
      (`SceneComponent.SetVisibility` _vertr true false :!label _label)
      (`SceneComponent.SetVisibility` _vert false false)
      (`SceneComponent.SetRelativeLocation` _vertr (+ (`SceneComponent.RelativeLocation` _vertr) (10.0 0.0 0.0)) false))
    (:`NewEnumerator2`
      (`SceneComponent.SetVisibility` _vertl true false :!label _label_2)
      (`SceneComponent.SetVisibility` _vert false false)
      (`SceneComponent.SetRelativeLocation` _vertl (+ (`SceneComponent.RelativeLocation` _vertl) (-10.0 0.0 0.0)) false))
    (:`NewEnumerator3`
      (goto _label))
    (:`NewEnumerator5`
      (goto _label_2))
    (:`NewEnumerator6`
      (goto _label))
    (:`NewEnumerator8`
      (goto _label_2))))