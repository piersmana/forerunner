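; Point hazard actor that occupies one WaveController grid cell at a set beat in a rhythm-timed level.
; The construction script snaps it to grid X/Z and beat Y in editor space, clamping the beat to at least the TimeSignature value.
; BeginPlay moves it to the runtime beat location and binds to AdvanceBeat.
; OnBeat sets cell collision on its downbeat, switches type on the off-beat, and clears it on the next downbeat.
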(event Custom|OnBeat
  (params (NewBeat :type Integer) (IsDownBeat :type Boolean))
  (bind _beat (Variables|Level|GetBeat))
  (bind _gridposition (Variables|Level|GetGridPosition))
  (bind _wavecontroller (Variables|Default|GetWaveController))
  (bind _returnvalue (== NewBeat _beat))
  (if (and _returnvalue IsDownBeat)
    (Default|SetGridCollision _wavecontroller _gridposition "NewEnumerator1")
    (elif (and IsDownBeat (== NewBeat (+ _beat 1)))
      (Default|ClearGridCollision _wavecontroller _gridposition "NewEnumerator2")
      (elif _returnvalue
        (Default|SetGridCollision _wavecontroller _gridposition "NewEnumerator2")))))

(event EventBeginPlay
  (bind _self self)
  (bind _wavecontroller (Variables|Default|GetWaveController))
  (bind _returnvalue (Transformation|GetActorLocation _self))
  (bind (_x _y _z) (Math|Vector|BreakVector _returnvalue))
  (EventDispatchers|BindEventtoAdvanceBeat _wavecontroller (delegate Custom|OnBeat))
  (bind _loc_y (Default|GetLocationfromBeat _wavecontroller (Variables|Level|GetBeat) false false))
  (Transformation|SetActorLocation (Math|Vector|MakeVector _x _loc_y _z) false))

(fn ConstructionScript
  (bind _returnvalue (Transformation|GetActorLocation))
  (bind (_x _y _z) (Math|Vector|BreakVector _returnvalue))
  (bind _outactors (Actor|GetAllActorsOfClass "/Game/Blueprints/WaveUtilities/WaveController.WaveController_C"))
  (bind _aswavecontroller_c (Utilities|Casting|CastToWaveController (Utilities|Array|Get(acopy) _outactors)))
  (Variables|Default|SetWaveController _aswavecontroller_c)
  (bind _gridposition (Default|GetGridfromLocation (Variables|Default|GetWaveController) _x _z))
  (bind _beat (Default|GetBeatfromLocation (Variables|Default|GetWaveController) _y true))
  (bind (_loc_x _loc_z) (Default|GetLocationfromGrid (Variables|Default|GetWaveController) _gridposition))
  (bind _loc_y (Default|GetLocationfromBeat (Variables|Default|GetWaveController) (Math|Integer|Max(Integer) _beat (Variables|/Game/Blueprints/WaveUtilities/WaveController.WaveController_C|GetTimeSignature (Variables|Default|GetWaveController))) false true))
  (if (!= (Math|Vector|MakeVector _loc_x _loc_y _loc_z) _returnvalue)
    (Transformation|SetActorLocation (Math|Vector|MakeVector _loc_x _loc_y _loc_z) false)
    (Variables|Level|SetGridPosition _gridposition)
    (Variables|Level|SetBeat (Math|Integer|Max(Integer) _beat (Variables|/Game/Blueprints/WaveUtilities/WaveController.WaveController_C|GetTimeSignature (Variables|Default|GetWaveController))))
    (else
      (bind (_loc_x_2 _loc_z_2) (Default|GetLocationfromGrid (Variables|Default|GetWaveController) (Variables|Level|GetGridPosition)))
      (bind _loc_y_2 (Default|GetLocationfromBeat (Variables|Default|GetWaveController) (Math|Integer|Max(Integer) (Variables|Level|GetBeat) (Variables|/Game/Blueprints/WaveUtilities/WaveController.WaveController_C|GetTimeSignature (Variables|Default|GetWaveController))) false true))
      (Transformation|SetActorLocation (Math|Vector|MakeVector _loc_x_2 _loc_y_2 _loc_z_2) false)
      (Variables|Level|SetBeat (Math|Integer|Max(Integer) (Variables|Level|GetBeat) (Variables|/Game/Blueprints/WaveUtilities/WaveController.WaveController_C|GetTimeSignature (Variables|Default|GetWaveController)))))))

(fn IsPlayerShip
  (params (CollidingObject :type Object%20Object%20Reference))
  (bind _returnvalue (Utilities|GetClass CollidingObject))
  (bind _returnvalue_2 (== _returnvalue "/Game/Blueprints/PlayerShip.PlayerShip_C"))
  (if _returnvalue_2
    (return _returnvalue_2)))

(fn SnapValue
  (params (Value :type Float%20%28single-precision%29) (Min :type Float%20%28single-precision%29) (Max :type Float%20%28single-precision%29) (Step :type Float%20%28single-precision%29))
  (bind _returnvalue (Math|Float|Clamp(Float) Value Min Max))
  (bind _returnvalue_2 (< Max 0.0))
  (bind _returnvalue_3 (Math|Float|Max(Float) Value Min))
  (bind _returnvalue_4 (Math|Float|SelectFloat _returnvalue_3 _returnvalue _returnvalue_2))
  (bind (_remainder _returnvalue_5) (Math|Float|Division(WholeandRemainder) _returnvalue_4 Step))
  (if (== _remainder 0.0)
    (LocalVariables|SetNewValue (* _returnvalue_5 Step))
    (elif (<= _remainder (/ Step 2.0))
      (LocalVariables|SetNewValue (* (+ _returnvalue_5 1) Step))
      (else
        (LocalVariables|SetNewValue (* (+ _returnvalue_5 -1) Step)))))
  (return (Math|Float|SelectFloat (Math|Float|Max(Float) (LocalVariables|GetNewValue) Min) (Math|Float|Clamp(Float) (LocalVariables|GetNewValue) Min Max) _returnvalue_2)))