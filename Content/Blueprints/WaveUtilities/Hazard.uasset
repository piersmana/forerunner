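; Beat-timed hazard that marks a pattern of cells in the WaveController's collision grid, offset from its root grid position.
; The construction script finds the WaveController, places the hazard by grid cell and beat, and attaches to it; BeginPlay recomputes Y for runtime.
; On beat callbacks it sets one collision type on its downbeat, another on its offbeat, and clears on the next downbeat.
; SnapValue is a step-rounding helper, not called here.
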(event Custom|OnBeat
  (params (NewBeat :type Integer) (IsDownBeat :type Boolean))
  (bind _beat (Variables|Level|GetBeat))
  (bind _gridcollision (Variables|Level|GetGridCollision))
  (bind _gridrootposition (Variables|Level|GetGridRootPosition))
  (bind _wavecontroller (Variables|Default|GetWaveController))
  (bind _returnvalue (== NewBeat _beat))
  (if (and _returnvalue IsDownBeat)
    (for _array_element _gridcollision
      (bind _new_grid_pos (Default|OffsetGridRoot _wavecontroller _array_element _gridrootposition))
      (Default|SetGridCollision _wavecontroller _new_grid_pos "NewEnumerator1"))
    (elif (and IsDownBeat (== NewBeat (+ _beat 1)))
      (for _array_element_2 _gridcollision
        (bind _new_grid_pos_2 (Default|OffsetGridRoot _wavecontroller _array_element_2 _gridrootposition))
        (Default|ClearGridCollision _wavecontroller _new_grid_pos_2 "NewEnumerator2"))
      (elif _returnvalue
        (for _array_element_3 _gridcollision
          (bind _new_grid_pos_3 (Default|OffsetGridRoot _wavecontroller _array_element_3 _gridrootposition))
          (Default|SetGridCollision _wavecontroller _new_grid_pos_3 "NewEnumerator2"))))))

(event EventBeginPlay
  (bind _self self)
  (bind _wavecontroller (Variables|Default|GetWaveController))
  (bind _returnvalue (Transformation|GetActorLocation _self))
  (bind (_x _y _z) (Math|Vector|BreakVector _returnvalue))
  (EventDispatchers|BindEventtoAdvanceBeat _wavecontroller (delegate Custom|OnBeat))
  (bind _loc_y (Default|GetLocationfromBeat _wavecontroller (Variables|Level|GetBeat) false false))
  (Transformation|SetActorLocation (Math|Vector|MakeVector _x _loc_y _z) false))

(fn ConstructionScript
  (Utilities|IsValid (Variables|Default|GetWaveController)
    (:Is%20Valid
      _)
    (:Is%20Not%20Valid
      (bind _outactors (Actor|GetAllActorsOfClass "/Game/Blueprints/WaveUtilities/WaveController.WaveController_C"))
      (bind _aswavecontroller_c (Utilities|Casting|CastToWaveController (Utilities|Array|Get(acopy) _outactors)))
      (Variables|Default|SetWaveController _aswavecontroller_c)))
  (bind (_loc_x _loc_z) (Default|GetLocationfromGrid (Variables|Default|GetWaveController) (Variables|Level|GetGridRootPosition)))
  (bind _loc_y (Default|GetLocationfromBeat (Variables|Default|GetWaveController) (Variables|Level|GetBeat) false true))
  (Transformation|SetActorLocation (Math|Vector|MakeVector _loc_x _loc_y _loc_z) false)
  (Class|Actor|AttachRootComponenttoActor (Variables|Default|GetWaveController) "None" "KeepWorldPosition"))

(fn SnapValue
  (params (Value :type Float%20%28single-precision%29) (Min :type Float%20%28single-precision%29) (Max :type Float%20%28single-precision%29) (Step :type Float%20%28single-precision%29))
  (bind _returnvalue (Math|Float|Clamp(Float) Value Min Max))
  (bind _returnvalue_2 (< Max 0.0))
  (bind _returnvalue_3 (Math|Float|Max(Float) Value Min))
  (bind _returnvalue_4 (Math|Float|SelectFloat _returnvalue_3 _returnvalue _returnvalue_2))
  (bind (_remainder _returnvalue_5) (Math|Float|Division(WholeandRemainder) _returnvalue_4 Step))
  (if (== _remainder 0.0)
    (LocalVariables|SetNewValue (* _returnvalue_5 Step))
    (elif (<= _remainder (/ Step 2.0))
      (LocalVariables|SetNewValue (* (+ _returnvalue_5 1) Step))
      (else
        (LocalVariables|SetNewValue (* (+ _returnvalue_5 -1) Step)))))
  (return (Math|Float|SelectFloat (Math|Float|Max(Float) (LocalVariables|GetNewValue) Min) (Math|Float|Clamp(Float) (LocalVariables|GetNewValue) Min Max) _returnvalue_2)))