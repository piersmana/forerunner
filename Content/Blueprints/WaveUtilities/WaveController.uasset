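; WaveController drives a rhythm-based flying level, moving itself along Y at a tempo-derived speed after Confirm starts play.
; It spawns set pieces from track length, opens difficulty and pause menus, broadcasts half-beat crossings and signals completion past the final hazard.
; SetTrack switches tempo variants, rescaling playback position to keep musical place.
; Helpers convert between beats, locations and a 3x3 X/Z grid with per-cell collision state.
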(event Custom|AdvanceBeat_Event
  (params (NewBeat :type Integer) (IsDownBeat :type Boolean))
  (if (not IsDownBeat)
    (Variables|LevelState|SetCurrentBeat NewBeat)))

(event EventBeginPlay
  (bind _leveltracks (Variables|Level|GetLevelTracks))
  (bind _item (Utilities|Array|Get(acopy) _leveltracks))
  (bind (_musictrack_6 _tempo_5) (Utilities|Struct|BreakMusicTempi _item))
  (Variables|Level|SetLevelBeats (Math|Float|Floor (* (/ (Math|Conversions|ToFloat(Integer) _tempo_5) 6e+01) (Variables|/Script/Engine.SoundBase|GetDuration _musictrack_6))))
  (for _index (range 0 (/ (Variables|Level|GetLevelBeats) (Math|Float|Floor (/ (Variables|LevelSet|GetSetPieceLength) (Variables|Globals|GetBeatLength)))))
    (Game|SpawnActorfromClass (Variables|LevelSet|GetLevelSetPiece) (Math|Transform|MakeTransform (Math|Vector|MakeVector 0.0 (* _index (Variables|LevelSet|GetSetPieceLength)) 0.0)) true))
  (bind _asmenuhud_c (Utilities|Casting|CastToMenuHUD (HUD|GetHUD (Game|GetPlayerController 0))))
  (Utilities|FlowControl|Delay 0.0001)
  (Default|OpenMenu _asmenuhud_c "/Game/Blueprints/MenuUtilities/Menus/Select_Difficulty_M.Select_Difficulty_M_C"))

(event Input|ActionEvents|InputActionConfirm
  (:Pressed
    (Utilities|FlowControl|DoOnce false
      (:Completed
        (bind _asflyingmode_c (Utilities|Casting|CastToFlyingMode (Game|GetGameMode)))
        (Variables|LevelState|SetCurrentDifficulty (Variables|/Game/Blueprints/FlyingMode.FlyingMode_C|GetDifficulty _asflyingmode_c))
        (EventDispatchers|BindEventtoAdvanceBeat (delegate Custom|AdvanceBeat_Event))
        (CallFunction|SetTrack (Variables|LevelState|GetCurrentDifficulty))
        (Default|CallBeginGameplay)
        (Variables|LevelState|SetForwardSpeed (CallFunction|GetPlayerSpeed))))))

(event Input|ActionEvents|InputActionPause
  (:Pressed
    (if (> (Math|Float|Absolute(Float) (Variables|LevelState|GetForwardSpeed)) 0.0)
      (bind _asmenuhud_c (Utilities|Casting|CastToMenuHUD (HUD|GetHUD (Game|GetPlayerController 0))))
      (Default|OpenMenu _asmenuhud_c "/Game/Blueprints/MenuUtilities/Menus/Pause_M.Pause_M_C"))))

(event EventTick
  (params (DeltaSeconds :type Float%20%28single-precision%29))
  (bind _returnvalue (Transformation|GetActorLocation))
  (bind _forwardspeed (Variables|LevelState|GetForwardSpeed))
  (bind (_x _y _z) (Math|Vector|BreakVector _returnvalue))
  (bind _returnvalue_2 (* DeltaSeconds _forwardspeed))
  (bind _returnvalue_3 (+ _returnvalue_2 _y))
  (if (< _forwardspeed 0.0)
    (bind (_beat _isdownbeat) (CallFunction|GetBeatfromLocation _y false))
    (bind (_beat_2 _isdownbeat_2) (CallFunction|GetBeatfromLocation _returnvalue_3 false))
    (if (or (!= _beat _beat_2) (Math|Boolean|NotEqual(Boolean) _isdownbeat _isdownbeat_2))
      (Default|CallAdvanceBeat _beat_2 _isdownbeat_2)
      (Default|CallAdvanceBeatB _beat_2 _isdownbeat_2)
      (if (> _beat_2 (Variables|Level|GetFinalHazardBeat))
        (Utilities|FlowControl|DoOnce false
          (:Completed
            (Default|CallLevelComplete)))))
    (Transformation|SetActorLocation (Math|Vector|MakeVector _x _returnvalue_3 _z) false)
    (Variables|LevelState|SetElapsedTime (+ (Variables|LevelState|GetElapsedTime) DeltaSeconds))))

(fn ConstructionScript)

(fn BeatstoSeconds
  (params (Beats :type Integer))
  (return (* Beats (/ 6e+01 (Math|Conversions|ToFloat(Integer) (Variables|LevelState|GetCurrentTempo))))))

(fn SecondstoBeats
  (params (Seconds :type Float%20%28single-precision%29))
  (return (Math|Float|Round (* (/ (Math|Conversions|ToFloat(Integer) (Variables|LevelState|GetCurrentTempo)) 6e+01) Seconds))))

(fn GetLocationfromGridValues
  (params (Grid%20X :type Integer) (Grid%20Z :type Integer))
  (bind _gridwidth (Variables|Globals|GetGridWidth))
  (return (* (Math|Integer|Clamp(Integer) Grid%20X -1 1) _gridwidth) (* (Math|Integer|Clamp(Integer) Grid%20Z -1 1) _gridwidth)))

(fn GetLocationfromBeat
  (params (Beat :type Integer) (IsOffBeat :type Boolean) (IsEditorLocation :type Boolean))
  (return (* (+ (* Beat 2) (Math|Integer|SelectInt -1 0 IsOffBeat)) (/ (Math|Float|SelectFloat (Variables|Globals|GetEditorBeatLength) (Variables|Globals|GetBeatLength) IsEditorLocation) 2.0))))

(fn GetBeatfromLocation
  (params (Loc%20Y :type Float%20%28single-precision%29) (IsEditorLocation :type Boolean))
  (bind _returnvalue (Math|Float|Absolute(Float) Loc%20Y))
  (bind _beatlength (Variables|Globals|GetBeatLength))
  (bind _editorbeatlength (Variables|Globals|GetEditorBeatLength))
  (bind _returnvalue_2 (Math|Float|SelectFloat _editorbeatlength _beatlength IsEditorLocation))
  (bind _returnvalue_3 (/ _returnvalue_2 2.0))
  (bind _returnvalue_4 (/ _returnvalue _returnvalue_3))
  (bind _returnvalue_5 (Math|Float|Floor _returnvalue_4))
  (bind _returnvalue_6 (Math|Integer|%(Integer) _returnvalue_5 2))
  (bind _returnvalue_7 (> _returnvalue_6 0))
  (return (+ (Math|Integer|SelectInt 1 0 _returnvalue_7) (/ _returnvalue_5 2)) _returnvalue_7))

(fn GetGridCollision
  (params (Grid%20Pos :type EGridPosition%20Enum :default "NewEnumerator0"))
  (return (Utilities|Array|Get(acopy) (Variables|LevelState|GetCollisionGrid) (CallFunction|GridtoCollision Grid%20Pos))))

(fn SetGridCollision
  (params (Grid%20Pos :type EGridPosition%20Enum :default "NewEnumerator0") (CollisionType :type EGridState%20Enum :default "NewEnumerator0"))
  (Utilities|Array|SetArrayElem (Variables|LevelState|GetCollisionGrid) (CallFunction|GridtoCollision Grid%20Pos) CollisionType))

(fn ClearGridCollision
  (params (Grid%20Loc :type EGridPosition%20Enum :default "NewEnumerator0") (CollisionState :type EGridState%20Enum :default "NewEnumerator0"))
  (bind _array_pos (CallFunction|GridtoCollision Grid%20Loc))
  (bind _collisiongrid (Variables|LevelState|GetCollisionGrid))
  (if (Utilities|Enum|Equal(Enum) (Utilities|Array|Get(acopy) _collisiongrid _array_pos) CollisionState)
    (Utilities|Array|SetArrayElem _collisiongrid _array_pos "NewEnumerator0")))

(fn GetGridValuesfromLocation
  (params (Loc%20X :type Float%20%28single-precision%29) (Loc%20Z :type Float%20%28single-precision%29))
  (bind _gridwidth (Variables|Globals|GetGridWidth))
  (return (Math|Float|Round (/ (Math|Float|Clamp(Float) Loc%20X (* _gridwidth -1.0) _gridwidth) _gridwidth)) (Math|Float|Round (/ (Math|Float|Clamp(Float) Loc%20Z (* _gridwidth -1.0) _gridwidth) _gridwidth))))

(fn GridValuestoName
  (params (Grid%20X :type Integer) (Grid%20Z :type Integer))
  (switch int Grid%20Z
    (:-1
      (switch int Grid%20X
        (:-1
          (LocalVariables|SetPosition "NewEnumerator8"))
        (:0
          (LocalVariables|SetPosition "NewEnumerator7"))
        (:1
          (LocalVariables|SetPosition "NewEnumerator6"))))
    (:0
      (switch int Grid%20X
        (:-1
          (LocalVariables|SetPosition "NewEnumerator5"))
        (:0
          (LocalVariables|SetPosition "NewEnumerator4"))
        (:1
          (LocalVariables|SetPosition "NewEnumerator3"))))
    (:1
      (switch int Grid%20X
        (:-1
          (LocalVariables|SetPosition "NewEnumerator2"))
        (:0
          (LocalVariables|SetPosition "NewEnumerator1"))
        (:1
          (LocalVariables|SetPosition "NewEnumerator0")))))
  (return (LocalVariables|GetPosition)))

(fn GridNametoValues
  (params (GridPosition :type EGridPosition%20Enum :default "NewEnumerator0"))
  (switch Utilities|FlowControl|Switch|SwitchonEGridPosition GridPosition
    (:NewEnumerator0
      (LocalVariables|SetX 1)
      (LocalVariables|SetZ 1))
    (:NewEnumerator1
      (LocalVariables|SetX 0)
      (LocalVariables|SetZ 1))
    (:NewEnumerator2
      (LocalVariables|SetX -1)
      (LocalVariables|SetZ 1))
    (:NewEnumerator3
      (LocalVariables|SetX 1)
      (LocalVariables|SetZ 0))
    (:NewEnumerator4
      (LocalVariables|SetX 0)
      (LocalVariables|SetZ 0))
    (:NewEnumerator5
      (LocalVariables|SetX -1)
      (LocalVariables|SetZ 0))
    (:NewEnumerator6
      (LocalVariables|SetX 1)
      (LocalVariables|SetZ -1))
    (:NewEnumerator7
      (LocalVariables|SetX 0)
      (LocalVariables|SetZ -1))
    (:NewEnumerator8
      (LocalVariables|SetX -1)
      (LocalVariables|SetZ -1)))
  (return (LocalVariables|GetX) (LocalVariables|GetZ)))

(fn GetLocationfromGrid
  (params (GridPosition :type EGridPosition%20Enum :default "NewEnumerator0"))
  (bind (_loc_x _loc_z) (CallFunction|GridNametoValues GridPosition))
  (bind (_loc_x_2 _loc_z_2) (CallFunction|GetLocationfromGridValues _loc_x _loc_z))
  (return _loc_x_2 _loc_z_2))

(fn GetGridfromLocation
  (params (Loc%20X :type Float%20%28single-precision%29) (Loc%20Z :type Float%20%28single-precision%29))
  (bind (_grid_x _grid_z) (CallFunction|GetGridValuesfromLocation Loc%20X Loc%20Z))
  (bind _gridposition (CallFunction|GridValuestoName _grid_x _grid_z))
  (return _gridposition))

(fn GridtoCollision
  (params (Grid%20Pos :type EGridPosition%20Enum :default "NewEnumerator0"))
  (return (Math|Conversions|ToInteger(Byte) Grid%20Pos)))

(fn IncreaseTempo
  (CallFunction|SetTrack (+ (Variables|LevelState|GetCurrentDifficulty) 1))
  (Variables|LevelState|SetForwardSpeed (CallFunction|GetPlayerSpeed)))

(fn ResetTempo
  (CallFunction|SetTrack (Variables|LevelState|GetCurrentDifficulty))
  (Variables|LevelState|SetForwardSpeed (CallFunction|GetPlayerSpeed)))

(fn GetPlayerSpeed
  (bind _seconds (CallFunction|BeatstoSeconds -1))
  (return (/ (Variables|Globals|GetBeatLength) _seconds)))

(fn SetTrack
  (params (TrackNum :type Integer))
  (bind _returnvalue (Class|GameplayStatics|GetAudioTimeSeconds))
  (bind _audio (Variables|Default|GetAudio))
  (bind _leveltracks (Variables|Level|GetLevelTracks))
  (bind _item (Utilities|Array|Get(acopy) _leveltracks TrackNum))
  (bind (_musictrack_6 _tempo_5) (Utilities|Struct|BreakMusicTempi _item))
  (if (== (Variables|LevelState|GetMusicStartTime) 0.0)
    (Variables|LevelState|SetMusicStartTime _returnvalue)
    (Variables|LevelState|SetMusicPosition (* (+ (- _returnvalue (Variables|LevelState|GetMusicStartTime)) (Variables|LevelState|GetMusicPosition)) (/ (Math|Conversions|ToFloat(Integer) (Variables|LevelState|GetCurrentTempo)) (Math|Conversions|ToFloat(Integer) _tempo_5))))
    (else
      (Variables|LevelState|SetMusicPosition (* (+ (- _returnvalue (Variables|LevelState|GetMusicStartTime)) (Variables|LevelState|GetMusicPosition)) (/ (Math|Conversions|ToFloat(Integer) (Variables|LevelState|GetCurrentTempo)) (Math|Conversions|ToFloat(Integer) _tempo_5))))
      (Variables|LevelState|SetMusicStartTime _returnvalue)))
  (Variables|LevelState|SetCurrentMusic _musictrack_6)
  (Variables|LevelState|SetCurrentTempo _tempo_5)
  (Audio|Components|Audio|SetSound _audio (Variables|LevelState|GetCurrentMusic))
  (Audio|Components|Audio|Play _audio (Variables|LevelState|GetMusicPosition))
  (return))

(fn OffsetGridRoot
  (params (Grid%20Pos :type EGridPosition%20Enum :default "NewEnumerator0") (OffsetRoot :type EGridPosition%20Enum :default "NewEnumerator0"))
  (bind (_loc_x _loc_z) (CallFunction|GridNametoValues Grid%20Pos))
  (bind (_loc_x_2 _loc_z_2) (CallFunction|GridNametoValues OffsetRoot))
  (bind _gridposition (CallFunction|GridValuestoName (Math|Integer|Clamp(Integer) (+ _loc_x _loc_x_2) -1 1) (Math|Integer|Clamp(Integer) (+ _loc_z _loc_z_2) -1 1)))
  (return _gridposition))

(fn StopTrack
  (params (StopAudio :type Boolean))
  (if StopAudio
    (Audio|Components|Audio|Stop (Variables|Default|GetAudio)))
  (Variables|LevelState|SetForwardSpeed 0.0))

(fn SetNewFinalHazard
  (params (Final%20Beat :type Integer))
  (if (> Final%20Beat (Variables|Level|GetFinalHazardBeat))
    (Variables|Level|SetFinalHazardBeat Final%20Beat)))